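; BP_StateComp is a component that tracks its owner's current mode as an enum with at least idle and equip states.
; Set and Is helpers for each mode wrap a shared ChangeType function and a comparison against the current type.
; ChangeType stores the previous type and fires OnStateTypeChanged with both old and new values, so listeners can react to transitions.
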(fn `ChangeType`
  (params (NewType :type "/Game/LSJ/State/EStateType Enum" :default "NewEnumerator0"))
  (locals (PrevType :type "/Game/LSJ/State/EStateType Enum"))
  (set `local.PrevType` (`self.Type`))
  (set `self.Type` NewType)
  (`self.OnStateTypeChanged` (`local.PrevType`) (`local.NewType`)))

(fn `IsEquipMode`
  (returns (ReturnValue :type Boolean))
  (return (`|EnumEquality` (`self.Type`) "NewEnumerator1")))

(fn `IsIdleMode`
  (returns (ReturnValue :type Boolean))
  (return (`|EnumEquality` (`self.Type`) "NewEnumerator0")))

(fn `SetEquipMode`
  (`self.ChangeType` "NewEnumerator1"))

(fn `SetIdleMode`
  (`self.ChangeType` "NewEnumerator0"))